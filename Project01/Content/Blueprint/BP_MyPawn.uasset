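; BP_MyPawn is a pawn that tests key, action and axis input mappings and provides basic camera-relative movement with mouse look.
; Enter, HelloWorld and AxisTest inputs print debug messages, while LookUp and Look_Right feed controller pitch and yaw.
; Move axes offset the actor along the player camera's forward and right vectors by fixed, unswept steps without delta-time scaling.
; Key01 increments Speed, which the movement code does not read.
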(event `self.ReceiveBeginPlay`)

(event `Key|Enter`
  (params (Key :type "Key Structure"))
  ;[1 1 1] Enter키 누르고 뗏을때 나오는 액터 매핑 설정
  (:`Pressed`
    (`KismetSystemLibrary.PrintString` "Enter Pressed" true true (struct :`G` 1.0 :`B` 0.049684 :`A` 1.0) 60.0))
  (:`Released`
    (`KismetSystemLibrary.PrintString` "Enter Released" true true (struct :`G` 0.016063 :`B` 1.0 :`A` 1.0) 60.0)))

(event `InputAction|HelloWorld`
  (params (Key :type "Key Structure"))
  ;[1 1 1] Enter키 누르고 뗏을때 나오는 액터 매핑 설정
  (:`Pressed`
    (`KismetSystemLibrary.PrintString` "HelloWorld Pressed" true true (struct :`G` 1.0 :`B` 0.049684 :`A` 1.0) 60.0))
  (:`Released`
    (`KismetSystemLibrary.PrintString` "HelloWorld Released" true true (struct :`G` 0.016063 :`B` 1.0 :`A` 1.0) 60.0)))

(event `InputAxis|AxisTest`
  (params (AxisValue :type "Float (single-precision)"))
  ;[1 1 1] Axis Test 눌리는지 확인작업 축 매핑
  (`KismetSystemLibrary.PrintString` (`KismetStringLibrary.Concat_StrStr` "Axis Test.." (`KismetStringLibrary.Conv_DoubleToString` AxisValue)) true true (struct :`G` 0.016063 :`B` 1.0 :`A` 1.0) 60.0))

(event `InputAxis|Move_Foward`
  (params (AxisValue :type "Float (single-precision)"))
  ;[1 1 1] 입력하는 키 셋팅
  ;[1 1 1] BP_MyPawn 을 앞뒤로 이동
  (`self.K2_AddActorWorldOffset` (* (`self.GetActorForwardVector` (`GameplayStatics.GetPlayerCameraManager` 0)) (* AxisValue 20.0))))

(event `InputAxis|Move_Right`
  (params (AxisValue :type "Float (single-precision)"))
  ;[1 1 1] 입력하는 키 셋팅
  ;[1 1 1] BP_MyPawn 을 좌우로 이동
  (`self.K2_AddActorWorldOffset` (* (`self.GetActorRightVector` (`GameplayStatics.GetPlayerCameraManager` 0)) (* AxisValue 40.0))))

(event `InputAxis|LookUp`
  (params (AxisValue :type "Float (single-precision)"))
  ;[1 1 1] 마우스 상하 셋팅
  (`self.AddControllerPitchInput` AxisValue))

(event `InputAction|Key01`
  (params (Key :type "Key Structure"))
  (:`Pressed`
    (set `self.Speed` (+ (`self.Speed`) 15.0))))

(event `InputAxis|Look_Right`
  (params (AxisValue :type "Float (single-precision)"))
  ;[1 1 1] 마우스 좌우 셋팅
  (`self.AddControllerYawInput` AxisValue))

(event `InputAction|Key02`
  (params (Key :type "Key Structure")))

(fn `UserConstructionScript`)