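; BP_MoveActor is an actor with a Sphere component and a function that moves it along local X while displaying a running counter.
; CountTimer scales its input into TotalDist, prints that as Korean-labelled minutes and seconds, and offsets the whole actor by the same step.
; Nothing here calls CountTimer: Tick is empty, and an older Sphere-only movement chain is left disconnected.
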(event `self.ReceiveTick`
  (params (DeltaSeconds :type "Float (single-precision)")))

(fn `Count Timer`
  (params (A :type "Float (double-precision)"))
  (bind _returnvalue (* A 20.0))
  ;[1 1 1] 1초당 걸리는 거리 셋팅
  (bind _output_get (set `self.TotalDist` (+ _returnvalue (`self.TotalDist`))))
  ;[1 1 1] 화면 문자 출력
  (`KismetSystemLibrary.PrintString` (`KismetStringLibrary.Concat_StrStr` (`KismetStringLibrary.Conv_IntToString` (`KismetMathLibrary.FFloor` (/ _output_get 60.0))) "분" (`KismetStringLibrary.Conv_IntToString` (`KismetMathLibrary.FFloor` (mod _output_get 60.0))) "초"))
  ;[1 1 1] Sphere 이동
  (`self.K2_AddActorLocalOffset` (`KismetMathLibrary.MakeVector` _returnvalue)))

(fn `UserConstructionScript`)